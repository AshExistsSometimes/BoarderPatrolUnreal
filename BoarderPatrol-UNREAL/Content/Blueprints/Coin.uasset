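; Coin pickup actor that spins in the level and awards score when the Snowball_Player touches it.
; On Cylinder overlap, it passes ScoreValue to SetScore on the BallGameInstance, plays its audio, then destroys itself after a short delay.
; Tick applies a frame-rate-independent local yaw rotation driven by RotationSpeed.
; Nothing disables the overlap during the delay, so re-entering can call SetScore again.
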(event OnComponentBeginOverlap(Cylinder)
  (params (OverlappedComponent :type Primitive%20Component%20Object%20Reference) (OtherActor :type Actor%20Object%20Reference) (OtherComp :type Primitive%20Component%20Object%20Reference) (OtherBodyIndex :type Integer) (bFromSweep :type Boolean) (SweepResult :type Hit%20Result%20Structure%20%28by%20ref%29))
  ;[1 1 1] Destroy Object & Score
  (Utilities|Casting|CastToSnowball_Player OtherActor)
  (bind _asball_game_instance (Utilities|Casting|CastToBallGameInstance (Game|GetGameInstance)))
  (Default|SetScore _asball_game_instance (Variables|Default|GetScoreValue))
  (Audio|Components|Audio|Play (Variables|Default|GetAudio) 0.0)
  (Utilities|FlowControl|Delay 0.3)
  (Actor|DestroyActor))

(event EventTick
  (params (DeltaSeconds :type Float%20%28single-precision%29))
  ;[1 1 1] Rotation
  (Transformation|AddActorLocalRotation (* (Math|Rotator|MakeRotator 0.0 0.0 (Variables|Default|GetRotationSpeed)) DeltaSeconds) false false))

(fn ConstructionScript)