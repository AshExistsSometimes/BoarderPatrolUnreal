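; BallBouncer is a bumper Blueprint that pushes a Ball away and plays a scale animation when its Cylinder is hit.
; A hit runs Bouncing, whose DoOnce gate resets only when the scale timeline finishes, after a successful Ball cast.
; HitReact applies an impulse at the impact point using negated world impact location times Force, leaving the normal unused.
; The timeline scales the Cylinder's X and Y from its captured scale.
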(event OnComponentHit(Cylinder)
  (params (HitComponent :type Primitive%20Component%20Object%20Reference) (OtherActor :type Actor%20Object%20Reference) (OtherComp :type Primitive%20Component%20Object%20Reference) (NormalImpulse :type Vector :default "0, 0, 0") (Hit :type Hit%20Result%20Structure%20%28by%20ref%29))
  (CallFunction|Bouncing OtherActor (.impactpoint Hit) (.impactnormal Hit)))

(event Custom|Bouncing
  (params (HitActor :type Actor%20Object%20Reference) (HitLocation :type Vector) (HItNormal :type Vector))
  (Utilities|FlowControl|DoOnce false :!label _label
    (:Completed
      (bind _asball (Utilities|Casting|CastToBall HitActor))
      (CallFunction|HitReact _asball HItNormal HitLocation)
      ;[1 1 1] Set Cylinder Initial Size
      (bind _output_get (Variables|Default|SetInitialScale (Variables|/Script/Engine.SceneComponent|GetRelativeScale3D (Variables|Default|GetCylinder))))
      ;[1 1 1] Animation Timeline / Set Scale
      (bind _newtrack_0 (Timeline|Timeline_0 PlayFromStart)
        (:Update
          (Transformation|SetRelativeScale3D (Variables|Default|GetCylinder) (Math|Vector|MakeVector (* _newtrack_0 (.x _output_get)) (* _newtrack_0 (.y _output_get)) (.z _output_get))))
        (:Finished
          (goto _label Reset))))))

(fn ConstructionScript)

(fn HitReact
  (params (Ball :type Ball%20Object%20Reference) (ImpactNormal :type Vector) (ImpactLocation :type Vector))
  (Physics|AddImpulseatLocation (Variables|/Game/Blueprints/Ball.Ball_C|GetMesh Ball) (* (* ImpactLocation -1.0) (Variables|Default|GetForce)) ImpactLocation "None"))